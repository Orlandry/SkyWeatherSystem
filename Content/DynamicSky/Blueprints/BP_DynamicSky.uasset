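; Dynamic sky actor that sets sun, moon, sky sphere, clouds and weather from TimeOfDay and a weather preset data asset.
; Construction script applies it all; weather changes update lighting, atmosphere, fog, player-attached Niagara effects, material parameter collection and invalidate RVT volumes.
; At BeginPlay, Sunny starts a timer alternating Snowy and Sunny presets, while Snowy or Rainy animate snow or puddle buildup.
; Tick's time-advance logic is disconnected.
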(event Custom|CustomEvent
  (Utilities|FlowControl|FlipFlop
    (:A
      (Variables|05-WeatherSetting|SetCurrentWeatherPreset "/Game/DynamicSky/DataAssets/DA_Snowy.DA_Snowy")
      (05-WeatherSetting|HandleWeatherSetting))
    (:B
      (Variables|05-WeatherSetting|SetCurrentWeatherPreset "/Game/DynamicSky/DataAssets/DA_Sunny.DA_Sunny")
      (05-WeatherSetting|HandleWeatherSetting))))

(event EventBeginPlay
  (05-WeatherSetting|HandleWeatherSetting)
  (Utilities|GetCurrentWeatherType
    (:Sunny
      (Utilities|Time|SetTimerbyEvent (delegate Custom|CustomEvent) 1e+01 true false 5.0))
    (:Snowy
      (Rendering|Material|SetScalarParameterValue "/Game/DynamicSky/Materials/MaterialParameterCollection/MPC_WeatherProperties.MPC_WeatherProperties" "SnowLevel" 0.0 :!class /Script/Engine.KismetMaterialLibrary)
      (Utilities|FlowControl|Delay 1.0)
      (Components|Timeline|SetPlayRate (Variables|Default|GetSnowCoverageAnimationTimeline) (/ 1.0 5.0))
      (bind _normalizefloattrack (Timeline|SnowCoverageAnimationTimeline Play)
        (:Update
          (Rendering|Material|SetScalarParameterValue "/Game/DynamicSky/Materials/MaterialParameterCollection/MPC_WeatherProperties.MPC_WeatherProperties" "SnowLevel" _normalizefloattrack :!class /Script/Engine.KismetMaterialLibrary))))
    (:Rainy
      (Rendering|Material|SetScalarParameterValue "/Game/DynamicSky/Materials/MaterialParameterCollection/MPC_WeatherProperties.MPC_WeatherProperties" "PuddleSize" 0.0 :!class /Script/Engine.KismetMaterialLibrary)
      (Utilities|FlowControl|Delay 1.0)
      (Components|Timeline|SetPlayRate (Variables|Default|GetPudleAnimationTimeline) (/ 1.0 15.0))
      (bind _normalizefloattrack_2 (Timeline|PudleAnimationTimeline Play)
        (:Update
          (Rendering|Material|SetScalarParameterValue "/Game/DynamicSky/Materials/MaterialParameterCollection/MPC_WeatherProperties.MPC_WeatherProperties" "PuddleSize" _normalizefloattrack_2 :!class /Script/Engine.KismetMaterialLibrary))))))

(event Collision|EventActorBeginOverlap
  (params (OtherActor :type Actor%20Object%20Reference)))

(event EventTick
  (params (DeltaSeconds :type Float%20%28single-precision%29)))

(fn ConstructionScript
  (bind _isdynmiskyspherevalid (01-BasicSettings|InitSkySphereMaterial))
  (if _isdynmiskyspherevalid
    (Utilities|FlowControl|Sequence
      (:then_0
        (05-WeatherSetting|HandleWeatherSetting))
      (:then_1
        (01-BasicSettings|HandleSunMoonRotation))
      (:then_2
        (01-BasicSettings|HandleVisibility))
      (:then_3
        (02-NightSettings|HandleNightSetting))
      (:then_4
        (03-CloudSettings|HandleCloudSetting)))))

(fn InitSkySphereMaterial
  (bind _returnvalue (Rendering|Material|CreateDynamicMaterialInstance (Variables|Default|GetSM_SkySphere) 0 "/Game/DynamicSky/Materials/Sky/MI_DynamicSkySphere.MI_DynamicSkySphere" "None" :!class /Script/Engine.PrimitiveComponent))
  (bind _output_get (Variables|Default|SetDynMI_SkySphere _returnvalue))
  (return (Utilities|IsValid _output_get)))

(fn HandleSunMoonRotation
  (bind _moondirectionallight (Variables|Default|GetMoonDirectionalLight))
  ;[1 1 1] Sun Rotation
  (Transformation|SetWorldRotation (Variables|Default|GetSunDirectionalLight) (Math|Rotator|MakeRotator 0.0 (Math|Float|MapRangeUnclamped (Variables|01-BasicSettings|GetTimeOfDay) (Variables|01-BasicSettings|GetDawnTime) (Variables|01-BasicSettings|GetDuskTime) 0.0 -1.8e+02) (Variables|01-BasicSettings|GetSunMoonRotation)) false false)
  ;[1 1 1] Moon Rotation
  (Transformation|SetWorldRotation _moondirectionallight (Math|Rotator|MakeRotator 0.0 (Math|Float|MapRangeUnclamped (Variables|01-BasicSettings|GetTimeOfDay) (Variables|01-BasicSettings|GetDuskTime) 24.0 0.0 -9e+01) (Variables|01-BasicSettings|GetSunMoonRotation)) false false)
  (Transformation|SetWorldRotation _moondirectionallight (Math|Rotator|MakeRotator 0.0 (Math|Float|MapRangeUnclamped (Variables|01-BasicSettings|GetTimeOfDay) 0.0 (Variables|01-BasicSettings|GetDawnTime) -9e+01 -1.8e+02) (Variables|01-BasicSettings|GetSunMoonRotation)) false false))

(fn HandleVisibility
  (Rendering|SetVisibility (Variables|Default|GetSunDirectionalLight) (Utilities|IsDayTime) false)
  (Rendering|SetVisibility (Variables|Default|GetMoonDirectionalLight) (Utilities|IsNightTime) false))

(fn HandleNightSetting
  (if (Utilities|IsNightTime)
    (Utilities|FlowControl|Sequence
      (:then_0
        (Rendering|Components|Light|SetIntensity (Variables|Default|GetMoonDirectionalLight) (Variables|02-NightSettings|GetMoonLightIntensity))
        (Rendering|Components|Light|SetLightColor (Variables|Default|GetMoonDirectionalLight) (Variables|02-NightSettings|GetMoonLightColor) true)
        (Class|DirectionalLightComponent|SetLightSourceAngle (Variables|Default|GetMoonDirectionalLight) (Variables|02-NightSettings|GetMoonLightSourceAngle))
        (Class|LightComponent|SetTemperature (Variables|Default|GetMoonDirectionalLight) (Variables|02-NightSettings|GetMoonLightTemperature)))
      (:then_1
        (Class|SkyAtmosphereComponent|SetRayleighScattering (Variables|Default|GetSkyAtmosphere) (Variables|02-NightSettings|GetNighttimeRayleighScattering))
        (Class|SkyAtmosphereComponent|SetMultiScatteringFactor (Variables|Default|GetSkyAtmosphere) (Variables|02-NightSettings|GetNighttimeMultiScattering)))
      (:then_2
        (Rendering|Material|SetScalarParameterValue (Variables|Default|GetDynMI_SkySphere) "IsStarVisible" (Math|Float|SelectFloat 1.0 0.0 (Variables|02-NightSettings|GetShouldShowStars)) :!class /Script/Engine.MaterialInstanceDynamic)
        (Rendering|Material|SetScalarParameterValue (Variables|Default|GetDynMI_SkySphere) "IsMoonVisible" (Math|Float|SelectFloat 1.0 0.0 (Variables|02-NightSettings|GetShouldShowMoon)) :!class /Script/Engine.MaterialInstanceDynamic)
        (Rendering|Material|SetVectorParameterValue (Variables|Default|GetDynMI_SkySphere) "MoonBasicSetting" (Utilities|Struct|MakeLinearColor (/ (Variables|02-NightSettings|GetMoonScale) 1e+01) (Variables|02-NightSettings|GetMoonRotation) (Variables|02-NightSettings|GetMoonBrightness) 1.0) :!class /Script/Engine.MaterialInstanceDynamic)
        (Rendering|Material|SetVectorParameterValue (Variables|Default|GetDynMI_SkySphere) "MoonTint" (Variables|02-NightSettings|GetMoonTint) :!class /Script/Engine.MaterialInstanceDynamic)))
    (else
      (05-WeatherSetting|HandleWeatherSetting)
      (Rendering|Material|SetScalarParameterValue (Variables|Default|GetDynMI_SkySphere) "IsStarVisible" 0.0 :!class /Script/Engine.MaterialInstanceDynamic)
      (Rendering|Material|SetScalarParameterValue (Variables|Default|GetDynMI_SkySphere) "IsMoonVisible" 0.0 :!class /Script/Engine.MaterialInstanceDynamic))))

(fn HandleCloudSetting
  (Utilities|GetCurrentWeatherType
    (:Sunny
      (switch Utilities|FlowControl|Switch|SwitchonECloudMode (Variables|03-CloudSettings|GetCurrentCloudMode)
        (:NewEnumerator0
          (Utilities|Toggle2DCloud false)
          (Utilities|ToggleVolumetricClouds false))
        (:NewEnumerator1
          (Utilities|ToggleVolumetricClouds false)
          (Utilities|Toggle2DCloud true)
          (Utilities|Set2DCloudSettingSunny))
        (:NewEnumerator2
          (Utilities|Toggle2DCloud false)
          (Utilities|ToggleVolumetricClouds true)
          (Utilities|SetVolumetricCloudsSetting))))
    (:Snowy
      (Utilities|Toggle2DCloud false)
      (Utilities|ToggleVolumetricClouds false))
    (:Rainy
      (Utilities|Toggle2DCloud true)
      (Utilities|ToggleVolumetricClouds false)
      (Utilities|Set2DCloudSettingRainy))))

(fn HandleWeatherSetting
  (Utilities|IsValid (Variables|Default|GetSnowNiagaraSystem)
    (:Is%20Valid
      (Components|Activation|Deactivate (Variables|Default|GetSnowNiagaraSystem))
      (Components|DestroyComponent (Variables|Default|GetSnowNiagaraSystem)))
    (:Is%20Not%20Valid
      (Utilities|IsValid (Variables|Default|GetRainNiagaraSystem)
        (:Is%20Valid
          (Components|Activation|Deactivate (Variables|Default|GetRainNiagaraSystem))
          (Components|DestroyComponent (Variables|Default|GetRainNiagaraSystem)))
        (:Is%20Not%20Valid
          _))
      (Utilities|IsValid (Variables|Default|GetLightningNS)
        (:Is%20Valid
          (Components|Activation|Deactivate (Variables|Default|GetLightningNS))
          (Components|DestroyComponent (Variables|Default|GetLightningNS)))
        (:Is%20Not%20Valid
          _))))
  (05-WeatherSetting|SetWeatherLightingProperties)
  (Utilities|ToggleSnow false)
  (Utilities|ToggleRain false)
  (Utilities|FlowControl|Sequence
    (:then_0
      (Utilities|GetCurrentWeatherType
        (:Snowy
          (Variables|01-BasicSettings|SetTimeOfDay 11.0)
          (Utilities|ToggleSnow true)
          (bind _returnvalue (Niagara|SpawnSystemAttached "/Game/DynamicSky/Niagara/Snow/NS_SnowStorm.NS_SnowStorm" (Variables|/Script/Engine.Actor|GetRootComponent (Game|GetPlayerCharacter 0)) "None" "0, 0, 0" "0, 0, 0" "KeepRelativeOffset" false))
          (Variables|Default|SetSnowNiagaraSystem _returnvalue))
        (:Rainy
          (Variables|01-BasicSettings|SetTimeOfDay 11.0)
          (Utilities|ToggleRain true)
          (bind _returnvalue_2 (Niagara|SpawnSystemAttached "/Game/DynamicSky/Niagara/Rain/NS_Rain.NS_Rain" (Variables|/Script/Engine.Actor|GetRootComponent (Game|GetPlayerCharacter 0)) "None" "0, 0, 0" "0, 0, 0" "KeepRelativeOffset" false))
          (Variables|Default|SetRainNiagaraSystem _returnvalue_2)
          (bind _returnvalue_3 (Niagara|SpawnSystemAttached "/Game/DynamicSky/Niagara/Lightning/NS_Lightning.NS_Lightning" (Variables|/Script/Engine.Actor|GetRootComponent (Game|GetPlayerCharacter 0)) "None" "0, 0, 0" "0, 0, 0" "KeepRelativeOffset" false))
          (Variables|Default|SetLightningNS _returnvalue_3))))
    (:then_1
      (Utilities|ForceUpdateRVT))))

(fn SetWeatherLightingProperties
  (bind _currentweatherpreset (Variables|05-WeatherSetting|GetCurrentWeatherPreset))
  (bind _exponentialheightfog (Variables|Default|GetExponentialHeightFog))
  (bind _sundirectionallight (Variables|Default|GetSunDirectionalLight))
  (bind _currentweatherpreset_2 (Variables|05-WeatherSetting|GetCurrentWeatherPreset))
  (bind _skyatmosphere (Variables|Default|GetSkyAtmosphere))
  (bind _currentweatherpreset_3 (Variables|05-WeatherSetting|GetCurrentWeatherPreset))
  (bind _direrectionallightsettings (Variables|/Game/DynamicSky/DataAssets/BP_WheatherData.BP_WheatherData_C|GetDirerectionalLightSettings _currentweatherpreset_2))
  (bind _exponentialheightfogsettings (Variables|/Game/DynamicSky/DataAssets/BP_WheatherData.BP_WheatherData_C|GetExponentialHeightFogSettings _currentweatherpreset))
  (bind _skyatmospheresettings (Variables|/Game/DynamicSky/DataAssets/BP_WheatherData.BP_WheatherData_C|GetSkyAtmosphereSettings _currentweatherpreset_3))
  (bind (_intensity _color _sourceangle _temperature) (Utilities|Struct|BreakS_DirectionalLightSettings _direrectionallightsettings))
  (bind (_multiscattering _rayleighscattering _miescatteringscale _mieabsorptionscale _mieanisotropy _aerialperspectiveviewdistancescale) (Utilities|Struct|BreakS_SkyAtmosphereSettings _skyatmospheresettings))
  (bind (_emissive _extinctionscale) (Utilities|Struct|BreakS_ExponentialHeightFogSettings _exponentialheightfogsettings))
  (if (Utilities|IsDayTime)
    (Utilities|FlowControl|Sequence
      (:then_0
        (Rendering|Components|Light|SetIntensity _sundirectionallight _intensity)
        (Rendering|Components|Light|SetLightColor _sundirectionallight _color true)
        (Class|DirectionalLightComponent|SetLightSourceAngle _sundirectionallight _sourceangle)
        (Class|LightComponent|SetTemperature _sundirectionallight _temperature))
      (:then_1
        (Rendering|Components|Light|SetIntensity (Variables|Default|GetSkyLight) (Utilities|Struct|BreakS_SkyLightSettings (Variables|/Game/DynamicSky/DataAssets/BP_WheatherData.BP_WheatherData_C|GetSkyLightSettings (Variables|05-WeatherSetting|GetCurrentWeatherPreset)))))
      (:then_2
        (Class|SkyAtmosphereComponent|SetMultiScatteringFactor _skyatmosphere _multiscattering)
        (Class|SkyAtmosphereComponent|SetRayleighScattering _skyatmosphere _rayleighscattering)
        (Class|SkyAtmosphereComponent|SetMieScatteringScale _skyatmosphere _miescatteringscale)
        (Class|SkyAtmosphereComponent|SetMieAbsorptionScale _skyatmosphere _mieabsorptionscale)
        (Class|SkyAtmosphereComponent|SetMieAnisotropy _skyatmosphere _mieanisotropy)
        (Class|SkyAtmosphereComponent|SetAerialPespectiveViewDistanceScale _skyatmosphere _aerialperspectiveviewdistancescale))
      (:then_3
        (Class|ExponentialHeightFogComponent|SetVolumetricFogEmissive _exponentialheightfog _emissive)
        (Class|ExponentialHeightFogComponent|SetVolumetricFogExtinctionScale _exponentialheightfog _extinctionscale)))))